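; BP_MainMenu is a VR main menu actor whose Play, Score and Exit options are chosen by shooting projectiles at box triggers.
; On BeginPlay it passes its three option meshes to the WBP_MainMenu widget.
; The boxes either destroy the menu and fire VRGameMode's game-start dispatcher, show the scoreboard, or quit.
; The scoreboard path lazily spawns BP_ScoreBoard, caches it on the game mode, refreshes it and hides the menu.
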(event OnComponentBeginOverlap(Box2)
  (params (OverlappedComponent :type Primitive%20Component%20Object%20Reference) (OtherActor :type Actor%20Object%20Reference) (OtherComp :type Primitive%20Component%20Object%20Reference) (OtherBodyIndex :type Integer) (bFromSweep :type Boolean) (SweepResult :type Hit%20Result%20Structure%20%28by%20ref%29))
  (if (== (Utilities|GetClass OtherActor) "/Game/DevelopedContent/Blueprint/VR_Projectile.VR_Projectile_C")
    (Game|QuitGame 0 "Quit")))

(event OnComponentBeginOverlap(Box)
  (params (OverlappedComponent :type Primitive%20Component%20Object%20Reference) (OtherActor :type Actor%20Object%20Reference) (OtherComp :type Primitive%20Component%20Object%20Reference) (OtherBodyIndex :type Integer) (bFromSweep :type Boolean) (SweepResult :type Hit%20Result%20Structure%20%28by%20ref%29))
  ;[1 1 1] Is projectile
  (if (== (Utilities|GetClass OtherActor) "/Game/DevelopedContent/Blueprint/VR_Projectile.VR_Projectile_C")
    (Actor|DestroyActor)
    (Default|CallGameStartEventDispatcher (.AsVRGame%20Mode (Utilities|Casting|CastToVRGameMode (Game|GetGameMode))))))

(event OnComponentBeginOverlap(Box1)
  (params (OverlappedComponent :type Primitive%20Component%20Object%20Reference) (OtherActor :type Actor%20Object%20Reference) (OtherComp :type Primitive%20Component%20Object%20Reference) (OtherBodyIndex :type Integer) (bFromSweep :type Boolean) (SweepResult :type Hit%20Result%20Structure%20%28by%20ref%29))
  (bind _returnvalue (Game|GetGameMode))
  (bind _asvrgame_mode (Utilities|Casting|CastToVRGameMode _returnvalue))
  (if (== (Utilities|GetClass OtherActor) "/Game/DevelopedContent/Blueprint/VR_Projectile.VR_Projectile_C")
    (Actor|DestroyActor OtherActor)
    (Utilities|IsValid (Variables|/Game/DevelopedContent/Blueprint/VRGameMode.VRGameMode_C|GetScoreBoard (.AsVRGame%20Mode (Utilities|Casting|CastToVRGameMode (Game|GetGameMode))))
      (:Is%20Valid
        _)
      (:Is%20Not%20Valid
        (bind _returnvalue_2 (Game|SpawnActorfromClass "/Game/Blueprints/BP_ScoreBoard.BP_ScoreBoard_C" (Math|Transform|MakeTransform (Variables|Default|GetScoreBoardLocation) "0.000000, 0, 0") "Undefined" 0 0))
        (Variables|/Game/DevelopedContent/Blueprint/VRGameMode.VRGameMode_C|SetScoreBoard _asvrgame_mode _returnvalue_2)))
    (Default|UpdateScoreBoard (.AsWBP%20Score%20Board (Utilities|Casting|CastToWBP_ScoreBoard (UserInterface|GetUserWidgetObject (Variables|/Game/Blueprints/BP_ScoreBoard.BP_ScoreBoard_C|GetScoreBoardWidgetComponent (Variables|/Game/DevelopedContent/Blueprint/VRGameMode.VRGameMode_C|GetScoreBoard _asvrgame_mode))))))
    (Rendering|SetActorHiddenInGame (Variables|/Game/DevelopedContent/Blueprint/VRGameMode.VRGameMode_C|GetMainMenu _asvrgame_mode) true)))

(event EventBeginPlay
  (bind _aswbp_main_menu (Utilities|Casting|CastToWBP_MainMenu (UserInterface|GetUserWidgetObject (Variables|Default|GetWidget))))
  (Variables|/Game/Widgets/WBP_MainMenu.WBP_MainMenu_C|SetPlayMesh _aswbp_main_menu (Variables|Default|GetPlayMesh))
  (Variables|/Game/Widgets/WBP_MainMenu.WBP_MainMenu_C|SetScoreMesh _aswbp_main_menu (Variables|Default|GetScoreMesh))
  (Variables|/Game/Widgets/WBP_MainMenu.WBP_MainMenu_C|SetExitMesh _aswbp_main_menu (Variables|Default|GetExitMesh)))

(event Collision|EventActorBeginOverlap
  (params (OtherActor :type Actor%20Object%20Reference)))

(event EventTick
  (params (DeltaSeconds :type Float%20%28single-precision%29)))

(fn ConstructionScript)