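; Enemy projectile actor that despawns after a set lifetime or after hitting the player's FirstPersonCharacter.
; BeginPlay starts a one-shot timer that destroys the actor when DestroyTime elapses.
; A Hit on that character class removes the sphere component, shows the particle system, then destroys the actor after a short delay and invokes CallKillCallback.
; Hits on other actor classes are ignored.
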(event Custom|DestroyAfterTime
  ;[1 1 1] Destroy Self After Some Time
  (Actor|DestroyActor))

(event EventBeginPlay
  ;[1 1 1] Destroy Self After Some Time
  (Utilities|Time|SetTimerbyEvent (delegate Custom|DestroyAfterTime) (Variables|Default|GetDestroyTime)))

(event Collision|EventHit
  (params (MyComp :type Primitive%20Component%20Object%20Reference) (Other :type Actor%20Object%20Reference) (OtherComp :type Primitive%20Component%20Object%20Reference) (bSelfMoved :type Boolean) (HitLocation :type Vector :default "0, 0, 0") (HitNormal :type Vector :default "0, 0, 0") (NormalImpulse :type Vector :default "0, 0, 0") (Hit :type Hit%20Result%20Structure%20%28by%20ref%29))
  ;[1 1 1] Destroy when hit with enemy
  (if (Utilities|ClassIsChildOf (Utilities|GetClass Other) "/Game/Blueprints/FirstPersonCharacter.FirstPersonCharacter_C")
    (Components|DestroyComponent (Variables|MyProjectile|GetSphere))
    (Rendering|SetVisibility (Variables|Default|GetParticleSystem) true false)
    (Utilities|FlowControl|Delay 1.0)
    (Actor|DestroyActor) ; Then destroy this projectile
    (Default|CallKillCallback)))

(fn ConstructionScript)