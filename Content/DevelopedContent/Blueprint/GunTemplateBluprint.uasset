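; Template VR gun that registers with an interface-implementing actor on contact, then handles trigger animation, firing and pull-to-reload.
; Tick fires through GunMode (single projectile or five-shot spread) with per-hand haptics, stopping after one shot when ObjectID is 0.
; Reloading projects hand movement onto the slide axis, adds haptics and sound, and refills ammo near full pull.
; Interface messages report ammo and reload-handle overlap to the interacting actor.
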(event OnComponentHit(GunMesh)
  (params (HitComponent :type Primitive%20Component%20Object%20Reference) (OtherActor :type Actor%20Object%20Reference) (OtherComp :type Primitive%20Component%20Object%20Reference) (NormalImpulse :type Vector :default "0, 0, 0") (Hit :type Hit%20Result%20Structure%20%28by%20ref%29))
  (if (Utilities|DoesObjectImplementInterface OtherActor "/Game/DevelopedContent/Blueprint/GunTemplateInterface.GunTemplateInterface_C")
    (if (not (Variables|Default|GetinHand))
      (Class|GunTemplateInterface|GunSend(Message) OtherActor (Utilities|GetObjectName OtherComp) (Variables|Default|GetObjectID) self (Variables|Default|GetGunMesh))
      (Class|GunTemplateInterface|ReturnAmmoSize(Message) OtherActor (Variables|Default|GetCurrentAmmoSize))
      (Variables|Default|SetAttachementActor0 OtherActor))))

(event OnComponentBeginOverlap(ReloadMesh)
  (params (OverlappedComponent :type Primitive%20Component%20Object%20Reference) (OtherActor :type Actor%20Object%20Reference) (OtherComp :type Primitive%20Component%20Object%20Reference) (OtherBodyIndex :type Integer) (bFromSweep :type Boolean) (SweepResult :type Hit%20Result%20Structure%20%28by%20ref%29))
  (if (Utilities|DoesObjectImplementInterface OtherActor "/Game/DevelopedContent/Blueprint/GunTemplateInterface.GunTemplateInterface_C")
    (if (Variables|Default|GetinHand)
      (Class|GunTemplateInterface|GunReloadCollision(Message) OtherActor true))))

(event OnComponentEndOverlap(ReloadMesh)
  (params (OverlappedComponent :type Primitive%20Component%20Object%20Reference) (OtherActor :type Actor%20Object%20Reference) (OtherComp :type Primitive%20Component%20Object%20Reference) (OtherBodyIndex :type Integer))
  (if (Utilities|DoesObjectImplementInterface OtherActor "/Game/DevelopedContent/Blueprint/GunTemplateInterface.GunTemplateInterface_C")
    (Class|GunTemplateInterface|GunReloadCollision(Message) OtherActor false)))

(event EventBeginPlay
  (Class|GunTemplateInterface|GunSend(Message) (stale OnComponentHit(GunMesh) OtherActor) (Utilities|GetObjectName (stale OnComponentHit(GunMesh) OtherComp)) (Variables|Default|GetObjectID) self (Variables|Default|GetGunMesh))
  (Class|GunTemplateInterface|ReturnAmmoSize(Message) (stale OnComponentHit(GunMesh) OtherActor) (Variables|Default|GetCurrentAmmoSize))
  (Variables|Default|SetAttachementActor0 (stale OnComponentHit(GunMesh) OtherActor)))

(event Collision|EventActorBeginOverlap
  (params (OtherActor :type Actor%20Object%20Reference)))

(event EventGunReceive
  (params (Hold :type Boolean) (TriggerAngle :type Float%20%28single-precision%29))
  (if Hold
    (Variables|Default|SetinHand Hold)
    (bind _output_get (Variables|Default|SetTriggerAngle TriggerAngle))
    (Transformation|SetRelativeRotation (Variables|Default|GetTriggerMesh) (Math|Rotator|MakeRotator 0.0 (* _output_get 35.0) 0.0) false false)))

(event EventTick
  (params (DeltaSeconds :type Float%20%28single-precision%29))
  (bind _reloadmove (Variables|Default|GetReloadMove))
  (bind _reloaddirection (Variables|Default|GetReloadDirection))
  (bind _returnvalue (Math|Float|Truncate _reloadmove))
  (if (Variables|Default|GetisReloading)
    (Transformation|SetWorldLocation (Variables|Default|GetReloadMesh) (+ (Transformation|GetWorldLocation _reloaddirection) (* (Math|Vector|Normalize (Math|Vector|GetForwardVector _reloaddirection)) _reloadmove)) false false)
    (if (>= _returnvalue (- (Math|Float|Truncate (Variables|Default|GetReloadLength)) 4))
      (Variables|Default|SetCurrentAmmoSize (Variables|Default|GetFullAmmoSize))
      (elif (!= (Math|Integer|%(Integer) _returnvalue 2) 0)
        (bind _newparam (CallFunction|SetVibrationHand (Variables|Default|GetHandID)))
        (Game|Feedback|ClientPlayForceFeedback (Game|GetPlayerController 0) _newparam false "None")
        (Audio|SpawnSoundatLocation "/Game/SoundsCrate-SciFi-PowerUp1.SoundsCrate-SciFi-PowerUp1" (Transformation|GetWorldLocation (Variables|Default|GetFireDirection)) "0, 0, 0" (* (/ _reloadmove 19.0) 1e+01) 1.0 0.0 "/Game/NewSoundAttenuation.NewSoundAttenuation")))
    (elif (Variables|Default|GetisFiring)
      (Utilities|FlowControl|Delay 0.1)
      (if (> (Variables|Default|GetCurrentAmmoSize) 0)
        (CallFunction|GunMode)
        (bind _newparam_2 (CallFunction|SetVibrationHand (Variables|Default|GetHandID)))
        (Game|Feedback|ClientPlayForceFeedback (Game|GetPlayerController 0) _newparam_2 false "None")
        (if (== (Variables|Default|GetObjectID) 0)
          (Variables|Default|SetisFiring false))))))

(event EventGunReloadUpdate
  (params (MoveDistance :type Float%20%28single-precision%29) (Current :type Vector) (Start :type Vector) (NewParam :type Actor%20Component%20Object%20Reference))
  (Variables|Default|SetReloadMove (Math|Float|Clamp(Float) (Math|Vector|DotProduct (- Current Start) (Math|Vector|GetForwardVector (Variables|Default|GetReloadDirection))) 0.0 (Variables|Default|GetReloadLength)))
  (Class|GunTemplateInterface|ReturnAmmoSize(Message) (Variables|Default|GetAttachementActor0) (Variables|Default|GetCurrentAmmoSize)))

(event EventGunReloading
  (params (Pulling :type Boolean))
  (bind _output_get (Variables|Default|SetisReloading Pulling))
  (if (not _output_get)
    (Transformation|SetWorldLocation (Variables|Default|GetReloadMesh) (Transformation|GetWorldLocation (Variables|Default|GetReloadDirection)) false false)
    (Variables|Default|SetReloadMove 0.0)))

(event EventGunFire
  (params (Fire :type Boolean) (NewParam :type Actor%20Component%20Object%20Reference))
  (Variables|Default|SetisFiring Fire))

(fn ConstructionScript
  (Variables|Default|SetCurrentAmmoSize (Variables|Default|GetFullAmmoSize)))

(fn SetVibrationHand
  (params (HandID :type Integer))
  (switch int HandID
    (:0
      (return "/Game/DevelopedContent/ForceFeedback/LeftForceFeedbackEffect.LeftForceFeedbackEffect"))
    (:1
      (return "/Game/DevelopedContent/ForceFeedback/RightForceFeedbackEffect.RightForceFeedbackEffect"))))

(fn GunMode
  (bind _firedirection (Variables|Default|GetFireDirection))
  (bind _returnvalue (Transformation|GetWorldLocation _firedirection))
  (bind _returnvalue_2 (Transformation|GetWorldRotation _firedirection))
  (bind _returnvalue_3 (Math|Transform|MakeTransform _returnvalue _returnvalue_2 "2.000000,2.000000,2.000000"))
  (switch int (Variables|Default|GetFireMode)
    (:0
      (bind _returnvalue_4 (Game|SpawnActorfromClass "/Game/DevelopedContent/Blueprint/VR_Projectile.VR_Projectile_C" _returnvalue_3 "AlwaysSpawn" 0 0))
      (Variables|/Game/DevelopedContent/Blueprint/VR_Projectile.VR_Projectile_C|SetparentActor _returnvalue_4 self)
      (Audio|PlaySoundatLocation "/Game/SoundsCrate-SciFi-Laser2.SoundsCrate-SciFi-Laser2" "0, 0, 0")
      (bind _result (Math|Integer|DecrementInt (Variables|Default|GetCurrentAmmoSize))
        (:%20%20
          (Variables|Default|SetCurrentAmmoSize _result)
          (Class|GunTemplateInterface|ReturnAmmoSize(Message) (Variables|Default|GetAttachementActor0) (Variables|Default|GetCurrentAmmoSize)))))
    (:1
      (for _index (range 0 4)
        (bind _returnvalue_5 (Game|SpawnActorfromClass "/Game/DevelopedContent/Blueprint/VR_Projectile.VR_Projectile_C" _returnvalue_3 "AlwaysSpawn" 0 0))
        (if (== _index 0)
          _
          (else
            (Game|Components|ProjectileMovement|SetVelocityinLocalSpace (Variables|/Game/DevelopedContent/Blueprint/VR_Projectile.VR_Projectile_C|GetProjectileMovement _returnvalue_5) (Math|Vector|MakeVector 2.5e+03 (Math|Random|RandomFloatinRange -5e+02 5e+02) (Math|Random|RandomFloatinRange -5e+02 5e+02)))))
        (Variables|/Game/DevelopedContent/Blueprint/VR_Projectile.VR_Projectile_C|SetparentActor _returnvalue_5 self))
      (Audio|PlaySoundatLocation "/Game/SoundsCrate-SciFi-Laser2.SoundsCrate-SciFi-Laser2" "0, 0, 0")
      (bind _result_2 (Math|Integer|DecrementInt (Variables|Default|GetCurrentAmmoSize))
        (:%20%20
          (Variables|Default|SetCurrentAmmoSize _result_2)
          (Class|GunTemplateInterface|ReturnAmmoSize(Message) (Variables|Default|GetAttachementActor0) (Variables|Default|GetCurrentAmmoSize)))))))