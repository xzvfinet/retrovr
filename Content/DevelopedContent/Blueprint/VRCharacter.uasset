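; VR player character with motion-controller gun handling, health and kill count.
; GunSend attaches weapons to the left hand; triggers drive left-gun firing, drop releasable items and start pull-to-reload, which Tick feeds with right-controller position.
; Gun messages update ammo, enemy projectile hits drain health toward game mode GameOver, and both show as scaled bars.
; Hand selection is hardwired left, with right-hand firing and several grab/drop branches disconnected.
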(event OnComponentHit(CapsuleComponent)
  (params (HitComponent :type Primitive%20Component%20Object%20Reference) (OtherActor :type Actor%20Object%20Reference) (OtherComp :type Primitive%20Component%20Object%20Reference) (NormalImpulse :type Vector :default "0, 0, 0") (Hit :type Hit%20Result%20Structure%20%28by%20ref%29))
  ;[1 1 1] LIFE DECREASE
  (if (== (Utilities|GetClass OtherActor) "/Game/Blueprints/EnemyProjectile.EnemyProjectile_C")
    (bind _asvrgame_mode (Utilities|Casting|CastToVRGameMode (Game|GetGameMode)))
    (if (Variables|/Game/DevelopedContent/Blueprint/VRGameMode.VRGameMode_C|GetGameRunning _asvrgame_mode)
      (if (< (Variables|Default|GetHealth_Count) 1)
        (bind _asvrgame_mode_2 (Utilities|Casting|CastToVRGameMode (Game|GetGameMode)))
        (Default|GameOver _asvrgame_mode_2)
        (else
          (bind _result (Math|Integer|DecrementInt (Variables|Default|GetHealth_Count))
            (:%20%20
              (Variables|Default|SetHealth_Count _result)
              (CallFunction|HealthUI))))))))

(event Custom|AddOneKill
  (bind _result (Math|Integer|IncrementInt (Variables|Default|GetEnemyKilled))
    (:%20%20
      (Rendering|Components|TextRender|SetText (Variables|Default|GetTextRender) (Utilities|Text|ToText(Integer) _result)))))

(event Custom|GoodShot
  (bind _output_get (Variables|Default|SetEnemyKilled (+ (Variables|Default|GetEnemyKilled) 1)))
  (Rendering|Components|TextRender|SetText (Variables|Default|GetTextRender) (Utilities|Text|ToText(Integer) _output_get)))

(event EventBeginPlay
  ;[1 1 1] Comment
  (Class|HeadMountedDisplayFunctionLibrary|SetTrackingOrigin "Floor")
  (Class|OculusFunctionLibrary|EnablePlayerCameraManagerFollowHmd true true))

(event EventReturnAmmoSize
  (params (AmmoCount :type Integer))
  (Variables|Default|SetAmmo_Count AmmoCount)
  (CallFunction|AmmoUI))

(event EventTick
  (params (DeltaSeconds :type Float%20%28single-precision%29))
  ;[1 1 1] Comment
  (if (Variables|Default|GetReloadPulling)
    (CallFunction|ReloadMovement (Variables|Default|GetPullingArm))))

(event EventGunReloadCollision
  (params (Colliding :type Boolean))
  (Variables|Default|SetReloadColliding Colliding))

(event EventGunSend
  (params (OtherName :type String) (ObjectID :type Integer) (CollidingActor :type Actor%20Object%20Reference) (CollidingMesh :type Static%20Mesh%20Component%20Object%20Reference))
  (bind (_motioncontroller _motioncontrollerstaticmesh _motioncontrollerarrow) (CallFunction|CheckHand OtherName))
  (Transformation|AttachComponentToComponent CollidingMesh _motioncontroller "None" "KeepWorld" "KeepWorld" "KeepWorld" true)
  (if (<= ObjectID 1)
    (Development|SetHiddeninGame _motioncontrollerstaticmesh true false)
    (Transformation|SetWorldTransform CollidingMesh (Math|Transform|MakeTransform (Transformation|GetWorldLocation _motioncontrollerstaticmesh) (Transformation|GetWorldRotation _motioncontrollerarrow) (Transformation|GetWorldScale CollidingMesh)) false false))
  (CallFunction|SetHoldingActorMesh OtherName CollidingActor CollidingMesh)
  (CallFunction|HealthUI)
  (CallFunction|AmmoUI))

(event Input|AxisEvents|InputAxisMoveForward
  (params (AxisValue :type Float%20%28single-precision%29))
  ;[1 1 1] Comment
  (Pawn|Input|AddMovementInput (Transformation|GetActorForwardVector) AxisValue false))

(event Input|AxisEvents|InputAxisMoveRight
  (params (AxisValue :type Float%20%28single-precision%29))
  ;[1 1 1] Comment
  (Pawn|Input|AddMovementInput (Transformation|GetActorRightVector) AxisValue false))

(event Input|KeyboardEvents|MotionControllerLeftTriggerAxis
  (params (AxisValue :type Float%20%28single-precision%29))
  (Class|GunTemplateInterface|GunReceive(Message) (Variables|Default|GetActorLeft) true AxisValue))

(event Input|KeyboardEvents|MotionControllerLeftShoulder
  (params (Key :type Key%20Structure :default "AnyKey")))

(event Input|KeyboardEvents|MotionControllerRightShoulder
  (params (Key :type Key%20Structure :default "AnyKey")))

(event Input|KeyboardEvents|F
  (params (Key :type Key%20Structure :default "AnyKey"))
  (:Pressed
    (Default|GameOver (.AsVRGame%20Mode (Utilities|Casting|CastToVRGameMode (Game|GetGameMode))))))

(event Input|KeyboardEvents|MotionControllerLeftTrigger
  (params (Key :type Key%20Structure :default "AnyKey"))
  (bind _leftwidgetinteraction (Variables|Default|GetLeftWidgetInteraction))
  (:Pressed
    (Class|WidgetInteractionComponent|PressPointerKey _leftwidgetinteraction "LeftMouseButton")
    (Variables|Default|SetLeftTriggerPressed true)
    (if (Variables|Default|GetisHoldingLeft)
      (Class|GunTemplateInterface|GunFire(Message) (Variables|Default|GetActorLeft) true)
      (bind _asgun_template_bluprint (Utilities|Casting|CastToGunTemplateBluprint (Variables|Default|GetActorLeft)))
      (Variables|/Game/DevelopedContent/Blueprint/GunTemplateBluprint.GunTemplateBluprint_C|SetHandID _asgun_template_bluprint 0)
      (elif (Variables|Default|GetisHoldingRight)
        (if (Variables|Default|GetReloadColliding)
          (Variables|Default|SetReloadHandInit (Transformation|GetWorldLocation (Variables|Default|GetMeshLeft)))
          (Variables|Default|SetReloadPulling true)
          (Variables|Default|SetPullingArm "Left")
          (Class|GunTemplateInterface|GunReloading(Message) (Variables|Default|GetActorRight) true)))))
  (:Released
    (Class|WidgetInteractionComponent|ReleasePointerKey _leftwidgetinteraction "LeftMouseButton")
    (Class|GunTemplateInterface|GunFire(Message) (Variables|Default|GetActorLeft) false)
    (Variables|Default|SetLeftTriggerPressed false)
    (if (Variables|Default|GetisHoldingLeft)
      (bind _asgun_template_bluprint_2 (Utilities|Casting|CastToGunTemplateBluprint (Variables|Default|GetActorLeft)))
      (if (> (Variables|/Game/DevelopedContent/Blueprint/GunTemplateBluprint.GunTemplateBluprint_C|GetObjectID _asgun_template_bluprint_2) 1)
        (Variables|/Game/DevelopedContent/Blueprint/GunTemplateBluprint.GunTemplateBluprint_C|SetinHand _asgun_template_bluprint_2 false)
        (Variables|Default|SetisHoldingLeft false)
        (Class|SceneComponent|DetachfromParent (Variables|Default|GetMeshInLeftHand) true true)
        (Physics|SetSimulatePhysics (Variables|Default|GetMeshInLeftHand) true)
        (Collision|SetCollisionEnabled (Variables|Default|GetMeshInLeftHand) "QueryAndPhysics")
        (Variables|Default|SetMeshInLeftHand 0)
        (Variables|Default|SetActorLeft 0))
      (else
        (Variables|Default|SetReloadPulling false)
        (Class|GunTemplateInterface|GunReloading(Message) (Variables|Default|GetActorRight) false)))))

(event Input|KeyboardEvents|MotionControllerRightTrigger
  (params (Key :type Key%20Structure :default "AnyKey"))
  (:Pressed
    (Variables|Default|SetRightTriggerPressed true)
    (if (Variables|Default|GetReloadColliding)
      (Variables|Default|SetReloadHandInit (Transformation|GetWorldLocation (Variables|Default|GetMeshRight)))
      (Variables|Default|SetReloadPulling true)
      (Variables|Default|SetPullingArm "Right")
      (Class|GunTemplateInterface|GunReloading(Message) (Variables|Default|GetActorLeft) true)))
  (:Released
    (Class|GunTemplateInterface|GunFire(Message) (Variables|Default|GetActorRight) false)
    (Variables|Default|SetRightTriggerPressed false)
    (if (Variables|Default|GetisHoldingRight)
      (bind _asgun_template_bluprint (Utilities|Casting|CastToGunTemplateBluprint (Variables|Default|GetActorRight)))
      (if (> (Variables|/Game/DevelopedContent/Blueprint/GunTemplateBluprint.GunTemplateBluprint_C|GetObjectID _asgun_template_bluprint) 1)
        (Variables|/Game/DevelopedContent/Blueprint/GunTemplateBluprint.GunTemplateBluprint_C|SetinHand _asgun_template_bluprint false)
        (Variables|Default|SetisHoldingRight false)
        (Class|SceneComponent|DetachfromParent (Variables|Default|GetMeshInRightHand) true true)
        (Physics|SetSimulatePhysics (Variables|Default|GetMeshInRightHand) true)
        (Collision|SetCollisionEnabled (Variables|Default|GetMeshInRightHand) "QueryAndPhysics")
        (Variables|Default|SetMeshInRightHand 0)
        (Variables|Default|SetActorRight 0))
      (else
        (Variables|Default|SetReloadPulling false)
        (Class|GunTemplateInterface|GunReloading(Message) (Variables|Default|GetActorLeft) false)))))

(fn ConstructionScript
  (Variables|Default|SetHealth_Count (Variables|Default|GetHealth_Max))
  (Variables|Default|SetAmmo_Count 0)
  (Rendering|Components|TextRender|SetText (Variables|Default|GetTextRender) (Utilities|Text|ToText(Integer) (Variables|Default|GetEnemyKilled))))

(fn CheckHand
  (params (Name :type String))
  (return (Variables|Default|GetLeftMC) (Variables|Default|GetMeshLeft) (Variables|Default|GetArrowLeft)))

(fn CheckTriggerPressed
  (params (Name :type String))
  (switch string Name
    (:MeshLeft
      (return (Variables|Default|GetLeftTriggerPressed) (Variables|Default|GetisHoldingLeft)))
    (:MeshRight
      (return (Variables|Default|GetRightTriggerPressed) (Variables|Default|GetisHoldingRight)))))

(fn SetHoldingActorMesh
  (params (Name :type String) (CollidingActor :type Actor%20Object%20Reference) (CollidingMesh :type Static%20Mesh%20Component%20Object%20Reference))
  (bind _output_get (Variables|Default|SetActorLeft CollidingActor))
  (Variables|Default|SetMeshInLeftHand 0)
  (Variables|Default|SetisHoldingLeft true)
  (bind _asgun_template_bluprint (Utilities|Casting|CastToGunTemplateBluprint _output_get))
  (Transformation|SetWorldTransform (Variables|Default|GetLeftCollisionBox) (Transformation|GetWorldTransform (Variables|/Game/DevelopedContent/Blueprint/GunTemplateBluprint.GunTemplateBluprint_C|GetAttachementCollisionBox0 _asgun_template_bluprint)) false false)
  (bind _asgun_template_bluprint_2 (Utilities|Casting|CastToGunTemplateBluprint CollidingActor))
  (Variables|/Game/DevelopedContent/Blueprint/GunTemplateBluprint.GunTemplateBluprint_C|SetinHand _asgun_template_bluprint_2 true)
  (bind _asgun_template_bluprint_3 (Utilities|Casting|CastToGunTemplateBluprint CollidingActor))
  (Variables|Default|SetAmmo_Max (Variables|/Game/DevelopedContent/Blueprint/GunTemplateBluprint.GunTemplateBluprint_C|GetFullAmmoSize _asgun_template_bluprint_3)))

(fn SetCollision
  (params (Set :type Boolean) (Name :type String))
  (if Set
    (switch string Name
      (:MeshLeft
        (Collision|SetCollisionEnabled (Variables|Default|GetMeshLeft) "QueryAndPhysics"))
      (:MeshRight
        (Collision|SetCollisionEnabled (Variables|Default|GetMeshRight) "QueryAndPhysics")))
    (else
      (switch string Name
        (:MeshLeft
          (Collision|SetCollisionEnabled (Variables|Default|GetMeshLeft) "NoCollision"))
        (:MeshRight
          (Collision|SetCollisionEnabled (Variables|Default|GetMeshRight) "NoCollision"))))))

(fn ReloadMovement
  (params (ArmName :type String))
  (Class|GunTemplateInterface|GunReloadUpdate(Message) (Variables|Default|GetActorLeft) 0.0 (Transformation|GetWorldLocation (Variables|Default|GetRightMC)) (Variables|Default|GetReloadHandInit)))

(fn HealthUI
  (Transformation|SetWorldScale3D (Variables|Default|GetUI_LifeBar) (Math|Vector|MakeVector 0.1 (* (/ (Math|Conversions|ToFloat(Integer) (Variables|Default|GetHealth_Count)) (Math|Conversions|ToFloat(Integer) (Variables|Default|GetHealth_Max))) 0.1) 0.1)))

(fn AmmoUI
  (Transformation|SetWorldScale3D (Variables|Default|GetUI_AmmoBar) (Math|Vector|MakeVector 0.1 (* (/ (Math|Conversions|ToFloat(Integer) (Variables|Default|GetAmmo_Count)) (Math|Conversions|ToFloat(Integer) (Variables|Default|GetAmmo_Max))) 0.1) 0.1)))