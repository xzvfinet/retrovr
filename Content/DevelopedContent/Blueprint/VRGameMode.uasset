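; VR game mode that handles game over and keeps a persistent kill-count high score list.
; BeginPlay loads the score list from a save slot or creates a new save object, and EndPlay writes it back.
; GameOver pauses the timer, removes the menu and enemies, shows the left interaction debug pointer and spawns a final-score actor.
; AddScore inserts ahead of the first tied or lower entry, never appending, and caps the list at seven.
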(event Custom|GameOver
  (bind _returnvalue (Game|GetGameMode))
  (bind _mainmenu (Variables|Default|GetMainMenu))
  (bind _asvrgame_mode (Utilities|Casting|CastToVRGameMode _returnvalue))
  (bind _timerhandle (Variables|VRGameMode_C|GetTimerHandle _asvrgame_mode))
  (if (Class|KismetSystemLibrary|TimerExistsHandle _timerhandle)
    (Utilities|Time|PauseTimerbyHandle _timerhandle))
  (if (Utilities|IsValid _mainmenu)
    (Actor|DestroyActor _mainmenu))
  (Variables|/Script/UMG.WidgetInteractionComponent|SetbShowDebug (Variables|/Game/DevelopedContent/Blueprint/VRCharacter.VRCharacter_C|GetLeftWidgetInteraction (.AsVRCharacter (Utilities|Casting|CastToVRCharacter (Game|GetPlayerCharacter 0)))) true)
  (Variables|Default|SetGameRunning false)
  (bind _outactors (Actor|GetAllActorsOfClass "/Game/Enemy/BaseEnemyPawn.BaseEnemyPawn_C"))
  (for _array_element _outactors
    (Actor|DestroyActor _array_element))
  (bind _returnvalue_2 (Game|SpawnActorfromClass "/Game/Blueprints/BP_GameOver.BP_GameOver_C" (Math|Transform|MakeTransform (Variables|Default|GetGameOverLocation) "0, 0, 0" "1,1.000000,1") "Undefined" 0 0))
  (bind _output_get (Variables|Default|SetGameOverActor _returnvalue_2))
  (Default|SetFinalScore _output_get (Variables|/Game/DevelopedContent/Blueprint/VRCharacter.VRCharacter_C|GetEnemyKilled (.AsVRCharacter (Utilities|Casting|CastToVRCharacter (Game|GetPlayerCharacter 0))))))

(event Custom|AddScore
  (params (Score :type ST%20Score%20Structure))
  (bind _scorelist (Variables|Default|GetScoreList))
  (bind (_array_element _array_index) (Utilities|Array|ForEachLoopwithBreak (Variables|Default|GetScoreList) :!label _label)
    (:LoopBody
      (if (>= (.KillNumber (Utilities|Struct|BreakST_Score Score)) (.KillNumber (Utilities|Struct|BreakST_Score _array_element)))
        (Utilities|Array|Insert (Variables|Default|GetScoreList) Score _array_index)
        (goto _label Break)))
    (:Completed
      (if (> (Utilities|Array|Length _scorelist) 7)
        (Utilities|Array|RemoveIndex _scorelist 7)))))

(event EventBeginPlay
  (bind _returnvalue (SaveGame|DoesSaveGameExist (Variables|Default|GetSlotName)))
  (if _returnvalue
    (bind _returnvalue_2 (SaveGame|LoadGamefromSlot (Variables|Default|GetSlotName)))
    (bind _output_get (Variables|Default|SetSaveGame (.AsBP%20Save%20Game (Utilities|Casting|CastToBP_SaveGame _returnvalue_2))))
    (Variables|Default|SetScoreList (Variables|/Game/Blueprints/BP_SaveGame.BP_SaveGame_C|GetScoreList _output_get))
    (else
      (bind _returnvalue_3 (SaveGame|CreateSaveGameObject "/Game/Blueprints/BP_SaveGame.BP_SaveGame_C"))
      (Variables|Default|SetSaveGame (.AsBP%20Save%20Game (Utilities|Casting|CastToBP_SaveGame _returnvalue_3))))))

(event EventTick
  (params (DeltaSeconds :type Float%20%28single-precision%29)))

(event EventEndPlay
  (params (EndPlayReason :type EEndPlayReason%20Enum :default "Destroyed"))
  (bind _savegame (Variables|Default|GetSaveGame))
  (Variables|/Game/Blueprints/BP_SaveGame.BP_SaveGame_C|SetScoreList _savegame (Variables|Default|GetScoreList))
  (SaveGame|SaveGametoSlot _savegame (Variables|Default|GetSlotName)))

(fn ConstructionScript)